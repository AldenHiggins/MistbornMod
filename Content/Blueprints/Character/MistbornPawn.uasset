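; MistbornPawn is a player pawn Blueprint that owns a push hand, a pull hand and holsters.
; Tick clamps CharacterMovement velocity to MaxSpeed.
; Spawn events create the left-style MistbornHand as PushHand, MistbornRightHand as PullHand, and holsters attached to the pawn.
; SetRecentlyFiredBullet links a fired MistbornProjectile to the push hand for left-hand shots, otherwise to the pull hand.
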(event EventTick
  (params (DeltaSeconds :type Float%20%28single-precision%29))
  (bind _charactermovement (Variables|Character|GetCharacterMovement))
  (|CallParentFunction DeltaSeconds)
  (if (>= (Math|Vector|VectorLength (Variables|/Script/Engine.MovementComponent|GetVelocity _charactermovement)) (Variables|Default|GetMaxSpeed))
    (Variables|/Script/Engine.MovementComponent|SetVelocity _charactermovement (* (Math|Vector|Normalize (Variables|/Script/Engine.MovementComponent|GetVelocity _charactermovement)) (Variables|Default|GetMaxSpeed)))))

(event EventSpawnHolsters
  (bind _returnvalue (Game|SpawnActorfromClass "/MistbornMod/Blueprints/Weapon/MistbornHolsters.MistbornHolsters_C" (Transformation|GetActorTransform) "Undefined" 0 self 0))
  (bind _output_get (Variables|Default|SetHolsters _returnvalue))
  (Transformation|AttachActorToActor _output_get self "None" "KeepWorld" "KeepWorld" "KeepWorld" false))

(event EventSpawnandRegisterHands
  (bind _returnvalue (Game|SpawnActorfromClass "/MistbornMod/Blueprints/Character/MistbornRightHand.MistbornRightHand_C" (Math|Transform|MakeTransform "0, 0, 0") "Undefined" self 0))
  (Variables|Default|SetPullHand _returnvalue)
  (bind _returnvalue_2 (Game|SpawnActorfromClass "/MistbornMod/Blueprints/Character/MistbornHand.MistbornHand_C" (Math|Transform|MakeTransform "0, 0, 0") "Undefined" self 0))
  (Variables|Default|SetPushHand _returnvalue_2))

(fn ConstructionScript
  (|CallParentFunction))

(fn SetRecentlyFiredBullet
  (params (Bullet :type Bullet%20Projectile%20Base%20Object%20Reference) (HandFiredFrom :type EControllerHand%20Enum))
  (bind _asmistborn_projectile (Utilities|Casting|CastToMistbornProjectile Bullet))
  (if (Utilities|Enum|Equal(Enum) (Utilities|String|EnumtoString HandFiredFrom) "Left")
    (Default|SetParentPushHand _asmistborn_projectile (Variables|Default|GetPushHand))
    (else
      (Default|SetParentPullHand _asmistborn_projectile (Variables|Default|GetPullHand)))))