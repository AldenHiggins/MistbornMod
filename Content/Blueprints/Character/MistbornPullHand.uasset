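; VR hand that pulls the player toward targets with a Mistborn-style metal pull while the trigger is held.
; Empty or holding a knife, it line-traces for an OdinCharacterBase and stores the hit in actor-local space, so the anchor follows that actor.
; With other held items, it pulls toward a reported bullet impact within range, scaling beam opacity, haptics and PullStrength by proximity.
; Both modes apply movement impulses and aim a blue beam.
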(event Custom|PulledBulletCollision
  (params (Hit%20Result :type Hit%20Result%20Structure))
  (Variables|Default|SetBulletHasCollided true)
  (Variables|Default|SetBulletCollisionPoint (.ImpactPoint (Collision|BreakHitResult Hit%20Result))))

(event EventBeginPlay
  (|CallParentFunction)
  (bind _returnvalue (Rendering|Material|CreateDynamicMaterialInstance (Variables|Default|GetBlueMetalBeam) 0 "/MistbornMod/Materials/MistbornLaser.MistbornLaser" :!class /Script/Engine.PrimitiveComponent))
  (Variables|Default|SetBeamMaterial _returnvalue))

(event EventTick
  (params (DeltaSeconds :type Float%20%28single-precision%29))
  (bind _controllermesh (Variables|Default|GetControllerMesh))
  (bind _grabbed_interaction_component (Variables|Default|GetGrabbed%20Interaction%20Component))
  (bind _returnvalue (Transformation|GetWorldLocation _controllermesh))
  (|CallParentFunction 0.0)
  (if (Variables|Default|GetTriggerPressed)
    (Utilities|IsValid _grabbed_interaction_component
      (:Is%20Valid
        (Utilities|Casting|CastToMistbornKnife (Components|GetOwner _grabbed_interaction_component)
          (:then
            (if (Variables|Default|GetPullAnchorFound) :!label _label
              (CallFunction|ApplyPullImpulse)
              (else
                (bind (_outhit _returnvalue_2) (Collision|LineTraceByChannel _returnvalue (+ _returnvalue (* (Math|Vector|GetForwardVector _controllermesh) 3e+03)) "TraceTypeQuery2" false (Utilities|Array|MakeArray (Variables|Default|GetPawn)) "None"))
                (if _returnvalue_2
                  (if (Utilities|ClassIsChildOf (Utilities|GetClass (.HitActor (Collision|BreakHitResult _outhit))) "/Game/Character/OdinCharacterBase.OdinCharacterBase_C")
                    (Variables|Default|SetPullAnchorPoint (Math|Transform|InverseTransformLocation (Transformation|GetActorTransform (.HitActor (Collision|BreakHitResult _outhit))) (.ImpactPoint (Collision|BreakHitResult _outhit))))
                    (Variables|Default|SetPullAnchorFound true)
                    (Variables|Default|SetPullAnchorActor (.HitActor (Collision|BreakHitResult _outhit)))
                    (else
                      (Rendering|SetVisibility (Variables|Default|GetBlueMetalBeam) false false :!label _label_2)))
                  (else
                    (goto _label_2))))))
          (:CastFailed
            (if (Variables|Default|GetBulletHasCollided)
              (CallFunction|ApplyPullImpulsetoBullet)
              (else
                (Variables|Default|SetPullStrength 0.0)
                (Rendering|Material|SetScalarParameterValue (Variables|Default|GetBeamMaterial) "LaserOpacity" 0.0 :!class /Script/Engine.MaterialInstanceDynamic))))))
      (:Is%20Not%20Valid
        (goto _label)))
    (else
      (Rendering|SetVisibility (Variables|Default|GetBlueMetalBeam) false false)
      (Variables|Default|SetPullStrength 0.0))))

(event EventTriggerPulled
  (bind _grabbed_interaction_component (Variables|Default|GetGrabbed%20Interaction%20Component))
  (Default|CallOnHandTriggerPulled)
  (if (Variables|Default|GetCanUseTrigger)
    (Variables|Default|SetTriggerPressed true)
    (Variables|Default|SetPullAnchorFound false)
    (Variables|Default|SetBulletHasCollided false)
    (Utilities|IsValid _grabbed_interaction_component
      (:Is%20Valid
        (Default|CallOnTriggerPulled _grabbed_interaction_component)))))

(event EventTriggerRelease
  (bind _grabbed_interaction_component (Variables|Default|GetGrabbed%20Interaction%20Component))
  (Default|CallOnHandTriggerReleased)
  (if (Variables|Default|GetCanUseTrigger)
    (Variables|Default|SetTriggerPressed false)
    (Variables|Default|SetPullAnchorFound false)
    (Variables|Default|SetBulletHasCollided false)
    (Utilities|IsValid _grabbed_interaction_component
      (:Is%20Valid
        (Default|CallOnTriggerReleased _grabbed_interaction_component)))))

(event EventHandHighlightInteractable
  (|CallParentFunction))

(fn ConstructionScript
  (|CallParentFunction))

(fn ApplyPullImpulse
  (bind _pullanchoractor (Variables|Default|GetPullAnchorActor))
  (bind _pullanchorpoint (Variables|Default|GetPullAnchorPoint))
  (bind _returnvalue (Transformation|GetActorTransform _pullanchoractor))
  (bind _returnvalue_2 (Math|Transform|TransformLocation _returnvalue _pullanchorpoint))
  (Physics|AddImpulse (Variables|/Script/Engine.Character|GetCharacterMovement (Variables|Default|GetPawn)) (* (Math|Vector|Normalize (- _returnvalue_2 (Transformation|GetWorldLocation (Variables|Default|GetControllerMesh)))) (Variables|Default|GetPullSpeed)) false)
  (Transformation|SetWorldRotation (Variables|Default|GetBlueMetalBeam) (Math|Rotator|FindLookatRotation (Transformation|GetWorldLocation (Variables|Default|GetControllerMesh)) _returnvalue_2) false false)
  (Rendering|SetVisibility (Variables|Default|GetBlueMetalBeam) true false))

(fn ApplyPullImpulsetoBullet
  (bind _maxpulldistance (Variables|Default|GetMaxPullDistance))
  (bind _bulletcollisionpoint (Variables|Default|GetBulletCollisionPoint))
  (bind _controllermesh (Variables|Default|GetControllerMesh))
  (bind _returnvalue (Transformation|GetWorldLocation _controllermesh))
  (bind _returnvalue_2 (- _bulletcollisionpoint _returnvalue))
  (bind _returnvalue_3 (Math|Vector|VectorLength _returnvalue_2))
  (bind _returnvalue_4 (/ _returnvalue_3 _maxpulldistance))
  (bind _returnvalue_5 (Math|Float|Clamp(Float) _returnvalue_4))
  (bind _returnvalue_6 (- 1.0 _returnvalue_5))
  (if (< _returnvalue_3 (Variables|Default|GetMaxPullDistance))
    (Physics|AddImpulse (Variables|/Script/Engine.Character|GetCharacterMovement (Variables|Default|GetPawn)) (* (Math|Vector|Normalize _returnvalue_2) (Variables|Default|GetPullSpeed)) false)
    (Transformation|SetWorldRotation (Variables|Default|GetBlueMetalBeam) (Math|Rotator|FindLookatRotation (Transformation|GetWorldLocation (Variables|Default|GetControllerMesh)) (Variables|Default|GetBulletCollisionPoint)) false false)
    (Rendering|SetVisibility (Variables|Default|GetBlueMetalBeam) true false)
    (Transformation|SetRelativeScale3D (Variables|Default|GetBlueMetalBeam) (Math|Vector|MakeVector _returnvalue_3 1.0 1.0))
    (Rendering|Material|SetScalarParameterValue (Variables|Default|GetBeamMaterial) "LaserOpacity" _returnvalue_6 :!class /Script/Engine.MaterialInstanceDynamic)
    (Class|PlayerController|PlayHapticEffect (Game|GetPlayerController 0) "/Game/Blueprint/Game/FX/ObjectGrabbed.ObjectGrabbed" (Variables|Default|GetHand) (* _returnvalue_6 2.0) false)
    (Variables|Default|SetPullStrength _returnvalue_6)
    (else
      (Variables|Default|SetPullStrength 0.0)
      (Rendering|Material|SetScalarParameterValue (Variables|Default|GetBeamMaterial) "LaserOpacity" 0.0 :!class /Script/Engine.MaterialInstanceDynamic))))