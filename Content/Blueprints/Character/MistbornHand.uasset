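; Motion-controller hand with a Mistborn-style push power and weapon gripping.
; Holding trigger pushes the highlighted skeletal mesh or bullet; after a bullet collision, it pushes the pawn away from the impact point.
; That recoil push fades with distance, as do beam opacity and haptics.
; Grabbing lerps the hand mesh onto the weapon after the grab pose settles; knife offset detaches it and repositions gun-derived weapons relative to the hand.
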(event Custom|PushedBulletCollision
  (params (FirstActor :type Actor%20Object%20Reference) (SecondActor :type Actor%20Object%20Reference) (HitPosition :type Vector) (HitResult :type Hit%20Result%20Structure))
  (Variables|Default|SetBulletHasCollided true)
  (Variables|Default|SetBulletCollisionPoint (.ImpactPoint (Collision|BreakHitResult HitResult))))

(event EventHandHighlightInteractable
  (|CallParentFunction))

(event EventBeginPlay
  ;[1 1 1] Begin Play
  (|CallParentFunction)
  (bind _returnvalue (Rendering|Material|CreateDynamicMaterialInstance (Variables|Default|GetBlueMetalBeam) 0 "/MistbornMod/Materials/MistbornLaser.MistbornLaser" :!class /Script/Engine.PrimitiveComponent))
  (Variables|Default|SetBeamMaterial _returnvalue))

(event EventTick
  (params (DeltaSeconds :type Float%20%28single-precision%29))
  (|CallParentFunction DeltaSeconds)
  (CallFunction|HandlePushLogic))

(event EventAttachHandtoGun
  (params (Attach :type Boolean) (Attach%20To%20component :type Scene%20Component%20Object%20Reference) (ScoeketName :type Name :default "None"))
  (bind _bone_to_center_to (Variables|Default|GetBone%20to%20center%20to))
  (bind _bone_to_grab (Variables|Default|GetBone%20To%20Grab))
  (bind _bone_to_grab_2 (Variables|Default|GetBone%20To%20Grab))
  (bind _component_to_grab (Variables|Default|GetComponent%20To%20Grab))
  (bind _component_to_grab_2 (Variables|Default|GetComponent%20To%20Grab))
  (bind _main_hand_mesh (Variables|Default|GetMain%20Hand%20Mesh))
  (bind _main_hand_mesh_2 (Variables|Default|GetMain%20Hand%20Mesh))
  (bind _returnvalue (Transformation|GetSocketTransform _main_hand_mesh _bone_to_center_to "RTS_Component"))
  (bind _returnvalue_2 (Math|Transform|InvertTransform _returnvalue))
  ;[1 1 1] Attach Hand mesh
  (if Attach
    (|EnsureHandHasValidPose_2)
    (if (== (Variables|Default|GetGrabbed%20Actor) (Components|GetOwner (Variables|Default|GetComponent%20To%20Grab)))
      (Transformation|DetachFromComponent _main_hand_mesh_2 "KeepWorld" "KeepWorld" "KeepWorld" true)
      (|SetLerpVariables_2)
      (Components|Timeline|SetPlayRate (Variables|Default|GetHand%20Lerp) (* (Variables|Default|GetPull%20Timeline%20PlayRate) 0.5))
      (bind (_direction _position) (Timeline|Timeline_0 PlayFromStart)
        (:Update
          (switch Utilities|FlowControl|Switch|SwitchonETimelineDirection _direction
            (:Forward
              (Variables|Default|SetHand%20Lerp%20to%20Transform (Math|Transform|MakeTransform (.location _returnvalue_2) (.rotation _returnvalue_2) (.scale (Variables|Default|GetHand%20Lerp%20from%20Transform))))
              (Transformation|SetWorldTransform (Variables|Default|GetMain%20Hand%20Mesh) (Math|Transform|Lerp(Transform) (Transformation|GetWorldTransform (Variables|Default|GetMain%20Hand%20Mesh)) (Math|Transform|MakeTransform (.location (Math|Transform|ComposeTransforms (Variables|Default|GetHand%20Lerp%20to%20Transform) (select (Transformation|DoesSocketExist _component_to_grab_2 _bone_to_grab) (Transformation|GetSocketTransform _component_to_grab_2 _bone_to_grab "RTS_World") (Transformation|GetWorldTransform (Variables|Default|GetComponent%20To%20Grab))))) (.rotation (Math|Transform|ComposeTransforms (Variables|Default|GetHand%20Lerp%20to%20Transform) (select (Transformation|DoesSocketExist _component_to_grab_2 _bone_to_grab) (Transformation|GetSocketTransform _component_to_grab_2 _bone_to_grab "RTS_World") (Transformation|GetWorldTransform (Variables|Default|GetComponent%20To%20Grab))))) "1,1,1") _position (Utilities|Select :Index _direction :Forward "QuatInterp" :Backward "EulerInterp")) false false))
            (:Backward
              (Transformation|SetRelativeTransform (Variables|Default|GetMain%20Hand%20Mesh) (Math|Transform|Lerp(Transform) (Variables|Default|GetHand%20Lerp%20from%20Transform) (Variables|Default|GetHand%20Lerp%20to%20Transform) _position (Utilities|Select :Index _direction :Forward "QuatInterp" :Backward "EulerInterp")) false false))))
        (:Finished
          (switch Utilities|FlowControl|Switch|SwitchonETimelineDirection _direction
            (:Forward
              (Transformation|AttachComponentToComponent _main_hand_mesh_2 _component_to_grab (select (Transformation|DoesSocketExist _component_to_grab _bone_to_grab_2) _bone_to_grab_2 "") "KeepWorld" "KeepWorld" "KeepWorld" false)
              (Variables|Default|SetAttachmentComplete true)
              (bind _asmistborn_knife (Utilities|Casting|CastToMistbornKnife (Variables|Default|GetGrabbed%20Actor)))
              (Variables|/MistbornMod/Blueprints/Weapon/MistbornKnife.MistbornKnife_C|SetCurrentKnifeOffset _asmistborn_knife 0.0)
              (Variables|/MistbornMod/Blueprints/Weapon/MistbornKnife.MistbornKnife_C|SetCurrentKnifePitch _asmistborn_knife 0.0))))))
    (elif (not (== (Transformation|GetAttachParent (Variables|Default|GetMain%20Hand%20Mesh)) (Variables|Default|GetScene1)))
      (Class|SceneComponent|Attachto (Variables|Default|GetMain%20Hand%20Mesh) (Variables|Default|GetScene1) "None" "KeepWorldPosition" false)
      (|SetLerpBackVariables_2)
      (Components|Timeline|SetPlayRate (Variables|Default|GetHand%20Lerp) (/ 2.0 (Class|GameplayStatics|GetGlobalTimeDilation)))
      (Timeline|Timeline_0 ReverseFromEnd))))

(event EventTriggerPulled
  (bind _grabbed_interaction_component (Variables|Default|GetGrabbed%20Interaction%20Component))
  ;[1 1 1] Trigger Logic
  (Default|CallOnHandTriggerPulled)
  (if (Variables|Default|GetCanUseTrigger)
    (Variables|Default|SetTriggerPressed true)
    (Variables|Default|SetBulletHasCollided false)
    (Utilities|IsValid _grabbed_interaction_component
      (:Is%20Valid
        (Default|CallOnTriggerPulled _grabbed_interaction_component)))))

(event EventTriggerRelease
  (bind _grabbed_interaction_component (Variables|Default|GetGrabbed%20Interaction%20Component))
  ;[1 1 1] Trigger Logic
  (Default|CallOnHandTriggerReleased)
  (if (Variables|Default|GetCanUseTrigger)
    (Variables|Default|SetTriggerPressed false)
    (Variables|Default|SetBulletHasCollided false)
    (Utilities|IsValid _grabbed_interaction_component
      (:Is%20Valid
        (Default|CallOnTriggerReleased _grabbed_interaction_component)))))

(event EventSetWeaponTransform
  (CallFunction|SetWeaponXForm))

(event EventRelease
  (|CallParentFunction)
  (Variables|Default|SetKnifeOffset "0, 0, 0")
  (Variables|Default|SetKnifePitch 0.0)
  (Variables|Default|SetAttachmentComplete false))

(event Input|KeyboardEvents|PageUp
  (params (Key :type Key%20Structure :default "AnyKey"))
  (bind _bone_to_center_to (Variables|Default|GetBone%20to%20center%20to))
  (bind _bone_to_grab (Variables|Default|GetBone%20To%20Grab))
  (bind _bone_to_grab_2 (Variables|Default|GetBone%20To%20Grab))
  (bind _component_to_grab (Variables|Default|GetComponent%20To%20Grab))
  (bind _component_to_grab_2 (Variables|Default|GetComponent%20To%20Grab))
  (bind _main_hand_mesh (Variables|Default|GetMain%20Hand%20Mesh))
  (bind _returnvalue (Transformation|GetSocketTransform _main_hand_mesh _bone_to_center_to "RTS_Component"))
  (bind _returnvalue_2 (Math|Transform|InvertTransform _returnvalue))
  ;[1 1 1] Attach Hand mesh
  (:Pressed
    (Class|SceneComponent|Attachto (Variables|Default|GetMain%20Hand%20Mesh) (Variables|Default|GetScene1) "None" "KeepWorldPosition" false)
    (|SetLerpBackVariables_2)
    (Components|Timeline|SetPlayRate (Variables|Default|GetHand%20Lerp) (/ 2.0 (Class|GameplayStatics|GetGlobalTimeDilation)))
    (bind (_direction _position) (Timeline|Timeline_0 ReverseFromEnd)
      (:Update
        (switch Utilities|FlowControl|Switch|SwitchonETimelineDirection _direction
          (:Forward
            (Variables|Default|SetHand%20Lerp%20to%20Transform (Math|Transform|MakeTransform (.location _returnvalue_2) (.rotation _returnvalue_2) (.scale (Variables|Default|GetHand%20Lerp%20from%20Transform))))
            (Transformation|SetWorldTransform (Variables|Default|GetMain%20Hand%20Mesh) (Math|Transform|Lerp(Transform) (Transformation|GetWorldTransform (Variables|Default|GetMain%20Hand%20Mesh)) (Math|Transform|MakeTransform (.location (Math|Transform|ComposeTransforms (Variables|Default|GetHand%20Lerp%20to%20Transform) (select (Transformation|DoesSocketExist _component_to_grab_2 _bone_to_grab) (Transformation|GetSocketTransform _component_to_grab_2 _bone_to_grab "RTS_World") (Transformation|GetWorldTransform (Variables|Default|GetComponent%20To%20Grab))))) (.rotation (Math|Transform|ComposeTransforms (Variables|Default|GetHand%20Lerp%20to%20Transform) (select (Transformation|DoesSocketExist _component_to_grab_2 _bone_to_grab) (Transformation|GetSocketTransform _component_to_grab_2 _bone_to_grab "RTS_World") (Transformation|GetWorldTransform (Variables|Default|GetComponent%20To%20Grab))))) "1,1,1") _position (Utilities|Select :Index _direction :Forward "QuatInterp" :Backward "EulerInterp")) false false))
          (:Backward
            (Transformation|SetRelativeTransform (Variables|Default|GetMain%20Hand%20Mesh) (Math|Transform|Lerp(Transform) (Variables|Default|GetHand%20Lerp%20from%20Transform) (Variables|Default|GetHand%20Lerp%20to%20Transform) _position (Utilities|Select :Index _direction :Forward "QuatInterp" :Backward "EulerInterp")) false false))))
      (:Finished
        (switch Utilities|FlowControl|Switch|SwitchonETimelineDirection _direction
          (:Forward
            (Transformation|AttachComponentToComponent (Variables|Default|GetMain%20Hand%20Mesh) _component_to_grab (select (Transformation|DoesSocketExist _component_to_grab _bone_to_grab_2) _bone_to_grab_2 "") "KeepWorld" "KeepWorld" "KeepWorld" false)
            (Variables|Default|SetAttachmentComplete true)
            (bind _asmistborn_knife (Utilities|Casting|CastToMistbornKnife (Variables|Default|GetGrabbed%20Actor)))
            (Variables|/MistbornMod/Blueprints/Weapon/MistbornKnife.MistbornKnife_C|SetCurrentKnifeOffset _asmistborn_knife 0.0)
            (Variables|/MistbornMod/Blueprints/Weapon/MistbornKnife.MistbornKnife_C|SetCurrentKnifePitch _asmistborn_knife 0.0)))))))

(fn ConstructionScript
  (|CallParentFunction))

(fn PushHighlightedObject
  (bind _controllermesh (Variables|Default|GetControllerMesh))
  (bind _highlighted_interaction_component (Variables|Default|GetHighlighted%20Interaction%20Component))
  (bind _pushstrength (Variables|Default|GetPushStrength))
  (bind _returnvalue (Components|GetOwner _highlighted_interaction_component))
  (bind _returnvalue_2 (Transformation|GetWorldLocation _controllermesh))
  (bind _returnvalue_3 (Actor|GetComponentsByClass _returnvalue "/Script/Engine.SkeletalMeshComponent"))
  (bind _returnvalue_4 (Transformation|GetActorLocation _returnvalue))
  (bind _returnvalue_5 (- _returnvalue_4 _returnvalue_2))
  (bind _returnvalue_6 (Math|Vector|Normalize _returnvalue_5))
  (bind _returnvalue_7 (* _returnvalue_6 _pushstrength))
  (Utilities|IsValid _highlighted_interaction_component
    (:Is%20Valid
      (if (> (Utilities|Array|Length _returnvalue_3) 0)
        (Physics|AddImpulse (Utilities|Array|Get(acopy) _returnvalue_3) _returnvalue_7 "None" false)
        (else
          (bind _asbase_bullet (Utilities|Casting|CastToBaseBullet _returnvalue))
          (Class|OdinProjectile|SetDisableSlowinginSlomoField _asbase_bullet true)
          (Class|OdinProjectile|SetProjectileVelocity _asbase_bullet _returnvalue_7))))))

(fn PushedBulletCollisionFunc
  (params (FirstActor :type Actor%20Object%20Reference) (SecondActor :type Actor%20Object%20Reference) (VectorInput :type Vector) (HitResult :type Hit%20Result%20Structure)))

(fn SetPushStrength
  (params (PushStrengthInput :type Float%20%28single-precision%29) (PushDistance :type Float%20%28single-precision%29))
  (bind _maxpushdistance (Variables|Default|GetMaxPushDistance))
  (bind _returnvalue (/ PushDistance _maxpushdistance))
  (bind _returnvalue_2 (Math|Float|Clamp(Float) _returnvalue))
  (bind _returnvalue_3 (- 1.0 _returnvalue_2))
  (Utilities|FlowControl|Sequence
    (:then_1
      (Rendering|Material|SetScalarParameterValue (Variables|Default|GetBeamMaterial) "LaserOpacity" _returnvalue_3 :!class /Script/Engine.MaterialInstanceDynamic))
    (:then_2
      (Class|PlayerController|PlayHapticEffect (Game|GetPlayerController 0) "/Game/Blueprint/Game/FX/ObjectGrabbed.ObjectGrabbed" (Variables|Default|GetHand) (* _returnvalue_3 2.0) false))))

(fn SetWeaponXForm
  (bind _returnvalue (Math|Rotator|MakeRotator 9e+01 -9e+01 0.0))
  (Utilities|IsValid (Variables|Default|GetGrabbed%20Actor)
    (:Is%20Valid
      (if (and (Variables|Default|GetGrip%20Complete) (Variables|Default|GetGripped))
        (if (and (not (Variables|Default|GetIs%20Secondary%20Grab)) (Class|OdinGrabInteractionComponent|GetPickUponGrab (Variables|Default|GetGrabbed%20Interaction%20Component)))
          (Utilities|FlowControl|Sequence
            (:then_0
              (bind _output_get (LocalVariables|SetIsPhysicsGrab (Utilities|IsValid (Class|PhysicsHandleComponent|GetGrabbedComponent (Variables|Default|GetWeaponPhysicsHandle)))))
              ;[1 1 1] Calculate Grabbed object transform
              (bind _output_get_2 (Variables|Default|SetNew%20Relative%20Transform (CallFunction|CalculateNewRelativeTransform _output_get)))
              (Variables|Default|SetNew%20World%20Transform (CallFunction|CalculateNewWorldTransform _output_get_2)))
            (:then_1
              (if (LocalVariables|GetIsPhysicsGrab)
                ;[1 1 1] Using physics handle, update that
                (Class|PhysicsHandleComponent|SetTargetLocationandRotation (Variables|Default|GetWeaponPhysicsHandle) (.Location (Math|Transform|BreakTransform (Variables|Default|GetNew%20World%20Transform))) (.Rotation (Math|Transform|BreakTransform (Variables|Default|GetNew%20World%20Transform))))
                (else
                  ;[1 1 1] Accounting for recoil on top of laggy hand transform
                  (bind _asgun_base (Utilities|Casting|CastToGun_Base (Variables|Default|GetGrabbed%20Actor))
                    (:then
                      (bind _newguntoworld (Default|ApplyRecoiltoTransform _asgun_base (Variables|Default|GetNew%20Relative%20Transform)))
                      (if (> (.X (Math|Vector|BreakVector (Variables|Default|GetKnifeOffset))) 0.0)
                        (Transformation|SetWorldTransform (VehicleSound|GetRootComponent _asgun_base) (Math|Transform|ComposeTransforms (Math|Transform|MakeTransform (Math|Vector|MakeVector 0.0 0.0 (* (.X (Math|Vector|BreakVector (Variables|Default|GetKnifeOffset))) -1.0)) (Math|Rotator|CombineRotators _returnvalue (Math|Vector|RotatorfromAxisandAngle (Math|Vector|GetRightVector _returnvalue) (Variables|Default|GetKnifePitch))) "1.000000,1.000000,1.000000") (Transformation|GetSocketTransform (Variables|Default|GetMain%20Hand%20Mesh) (Variables|Default|GetBone%20to%20center%20to) "RTS_World")) false false)
                        (else
                          (Transformation|SetRelativeTransform (VehicleSound|GetRootComponent _asgun_base) _newguntoworld false false))))
                    (:CastFailed
                      ;[1 1 1] Not using physics, but not a gun; just set position
                      (Transformation|SetActorTransform (Variables|Default|GetGrabbed%20Actor) (Variables|Default|GetNew%20World%20Transform)))))))
            (:then_2
              (Default|CallOnHandPositionUpdated))))))))

(fn DetachWeapon
  (Class|SceneComponent|Attachto (Variables|Default|GetMain%20Hand%20Mesh) (Variables|Default|GetScene1) "None" "KeepWorldPosition" false))

(fn HandlePushLogic
  (bind _bulletcollisionpoint (Variables|Default|GetBulletCollisionPoint))
  (bind _controllermesh (Variables|Default|GetControllerMesh))
  (bind _maxpushdistance (Variables|Default|GetMaxPushDistance))
  (bind _returnvalue (Transformation|GetWorldLocation _controllermesh))
  (bind _returnvalue_2 (- _bulletcollisionpoint _returnvalue))
  (bind _returnvalue_3 (Math|Vector|VectorLength _returnvalue_2))
  (bind _returnvalue_4 (/ _returnvalue_3 _maxpushdistance))
  (bind _returnvalue_5 (- 1.0 _returnvalue_4))
  (bind _returnvalue_6 (Math|Float|Max(Float) _returnvalue_5 0.0))
  (if (Variables|Default|GetTriggerPressed)
    (if (Variables|Default|GetBulletHasCollided)
      (Physics|AddImpulse (Variables|/Script/Engine.Character|GetCharacterMovement (Variables|Default|GetPawn)) (* (Math|Vector|Normalize _returnvalue_2) (* (Variables|Default|GetPushStrength) -1.0 _returnvalue_6)) false)
      (CallFunction|SetPushStrength _returnvalue_6 _returnvalue_3)
      (Transformation|SetWorldRotation (Variables|Default|GetBlueMetalBeam) (Math|Rotator|FindLookatRotation (Transformation|GetWorldLocation (Variables|Default|GetControllerMesh)) (Variables|Default|GetBulletCollisionPoint)) false false)
      (Rendering|SetVisibility (Variables|Default|GetBlueMetalBeam) true false)
      (Transformation|SetRelativeScale3D (Variables|Default|GetBlueMetalBeam) (Math|Vector|MakeVector _returnvalue_3 1.0 1.0))
      (else
        (Utilities|IsValid (Variables|Default|GetHighlighted%20Interaction%20Component)
          (:Is%20Valid
            (CallFunction|PushHighlightedObject)))))
    (else
      (Rendering|SetVisibility (Variables|Default|GetBlueMetalBeam) false false)
      (CallFunction|SetPushStrength 0.0 (Variables|Default|GetMaxPushDistance)))))

(fn SetKnifeOffset
  (params (NewOffset :type Float%20%28single-precision%29) (NewPitch :type Float%20%28single-precision%29))
  (if (Variables|Default|GetAttachmentComplete)
    (Utilities|FlowControl|Sequence
      (:then_0
        (Variables|Default|SetKnifeOffset (Math|Vector|MakeVector NewOffset 0.0 0.0)))
      (:then_1
        (Variables|Default|SetKnifePitch NewPitch))
      (:then_2
        (if (> NewOffset 0.0)
          (CallFunction|DetachWeapon)
          (else
            (CallFunction|AttachWeapon)))))))

(fn AttachWeapon
  (Variables|Default|SetKnifePitch 0.0)
  (CallFunction|SetWeaponXForm)
  (Transformation|AttachComponentToComponent (Variables|Default|GetMain%20Hand%20Mesh) (Variables|Default|GetComponent%20To%20Grab) (Utilities|String|StringToName (Utilities|String|MakeLiteralString "LeftGrabSocket")) "KeepWorld" "KeepWorld" "KeepWorld" false))