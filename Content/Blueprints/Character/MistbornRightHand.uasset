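; VR right-hand Blueprint for the Mistborn character that grips weapons and lets the trigger pull the player through the world.
; With a knife or empty hand it traces for a character to anchor on; otherwise it pulls toward a reported bullet impact, with a blue beam and, for bullets, distance-scaled haptics.
; A timeline lerps the hand mesh onto grabbed weapons once the grip pose is ready, while transform updates handle physics grips, gun recoil and knife offset.
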(event Custom|PulledBulletCollision
  (params (Hit%20Result :type Hit%20Result%20Structure))
  (Variables|Default|SetBulletHasCollided_0 true)
  (Variables|Default|SetBulletCollisionPoint_0 (.ImpactPoint (Collision|BreakHitResult Hit%20Result))))

(event EventBeginPlay
  (|CallParentFunction)
  (bind _returnvalue (Rendering|Material|CreateDynamicMaterialInstance (Variables|Default|GetBlueMetalBeam_0) 0 "/MistbornMod/Materials/MistbornLaser.MistbornLaser" :!class /Script/Engine.PrimitiveComponent))
  (Variables|Default|SetBeamMaterial_0 _returnvalue))

(event EventTick
  (params (DeltaSeconds :type Float%20%28single-precision%29))
  (|CallParentFunction 0.0)
  (CallFunction|HandlePullLogic))

(event EventAttachHandtoGun
  (params (Attach :type Boolean) (Attach%20To%20component :type Scene%20Component%20Object%20Reference) (ScoeketName :type Name :default "None"))
  (bind _bone_to_center_to (Variables|Default|GetBone%20to%20center%20to))
  (bind _bone_to_grab (Variables|Default|GetBone%20To%20Grab))
  (bind _bone_to_grab_2 (Variables|Default|GetBone%20To%20Grab))
  (bind _component_to_grab (Variables|Default|GetComponent%20To%20Grab))
  (bind _component_to_grab_2 (Variables|Default|GetComponent%20To%20Grab))
  (bind _main_hand_mesh (Variables|Default|GetMain%20Hand%20Mesh))
  (bind _main_hand_mesh_2 (Variables|Default|GetMain%20Hand%20Mesh))
  (bind _returnvalue (Transformation|GetSocketTransform _main_hand_mesh _bone_to_center_to "RTS_Component"))
  (bind _returnvalue_2 (Math|Transform|InvertTransform _returnvalue))
  ;[1 1 1] Attach Hand mesh
  (if Attach
    (|EnsureHandHasValidPose_2_2)
    (if (== (Variables|Default|GetGrabbed%20Actor) (Components|GetOwner (Variables|Default|GetComponent%20To%20Grab)))
      (Transformation|DetachFromComponent _main_hand_mesh_2 "KeepWorld" "KeepWorld" "KeepWorld" true)
      (|SetLerpVariables_2_2)
      (Components|Timeline|SetPlayRate (Variables|Default|GetHand%20Lerp) (* (Variables|Default|GetPull%20Timeline%20PlayRate) 0.5))
      (bind (_direction _position) (Timeline|Timeline_0 PlayFromStart)
        (:Update
          (switch Utilities|FlowControl|Switch|SwitchonETimelineDirection _direction
            (:Forward
              (Variables|Default|SetHand%20Lerp%20to%20Transform (Math|Transform|MakeTransform (.location _returnvalue_2) (.rotation _returnvalue_2) (.scale (Variables|Default|GetHand%20Lerp%20from%20Transform))))
              (Transformation|SetWorldTransform (Variables|Default|GetMain%20Hand%20Mesh) (Math|Transform|Lerp(Transform) (Transformation|GetWorldTransform (Variables|Default|GetMain%20Hand%20Mesh)) (Math|Transform|MakeTransform (.location (Math|Transform|ComposeTransforms (Variables|Default|GetHand%20Lerp%20to%20Transform) (select (Transformation|DoesSocketExist _component_to_grab_2 _bone_to_grab) (Transformation|GetSocketTransform _component_to_grab_2 _bone_to_grab "RTS_World") (Transformation|GetWorldTransform (Variables|Default|GetComponent%20To%20Grab))))) (.rotation (Math|Transform|ComposeTransforms (Variables|Default|GetHand%20Lerp%20to%20Transform) (select (Transformation|DoesSocketExist _component_to_grab_2 _bone_to_grab) (Transformation|GetSocketTransform _component_to_grab_2 _bone_to_grab "RTS_World") (Transformation|GetWorldTransform (Variables|Default|GetComponent%20To%20Grab))))) "1,1,1") _position (Utilities|Select :Index _direction :Forward "QuatInterp" :Backward "EulerInterp")) false false))
            (:Backward
              (Transformation|SetRelativeTransform (Variables|Default|GetMain%20Hand%20Mesh) (Math|Transform|Lerp(Transform) (Variables|Default|GetHand%20Lerp%20from%20Transform) (Variables|Default|GetHand%20Lerp%20to%20Transform) _position (Utilities|Select :Index _direction :Forward "QuatInterp" :Backward "EulerInterp")) false false))))
        (:Finished
          (switch Utilities|FlowControl|Switch|SwitchonETimelineDirection _direction
            (:Forward
              (Transformation|AttachComponentToComponent _main_hand_mesh_2 _component_to_grab (select (Transformation|DoesSocketExist _component_to_grab _bone_to_grab_2) _bone_to_grab_2 "") "KeepWorld" "KeepWorld" "KeepWorld" false)
              (Variables|Default|SetAttachmentComplete true)
              (bind _asmistborn_knife (Utilities|Casting|CastToMistbornKnife (Variables|Default|GetGrabbed%20Actor)))
              (Variables|/MistbornMod/Blueprints/Weapon/MistbornKnife.MistbornKnife_C|SetCurrentKnifeOffset _asmistborn_knife 0.0)
              (Variables|/MistbornMod/Blueprints/Weapon/MistbornKnife.MistbornKnife_C|SetCurrentKnifePitch _asmistborn_knife 0.0))))))
    (elif (not (== (Transformation|GetAttachParent (Variables|Default|GetMain%20Hand%20Mesh)) (Variables|Default|GetScene1)))
      (Class|SceneComponent|Attachto (Variables|Default|GetMain%20Hand%20Mesh) (Variables|Default|GetScene1) "None" "KeepWorldPosition" false)
      (|SetLerpBackVariables_2_2)
      (Components|Timeline|SetPlayRate (Variables|Default|GetHand%20Lerp) (/ 2.0 (Class|GameplayStatics|GetGlobalTimeDilation)))
      (Timeline|Timeline_0 ReverseFromEnd))))

(event EventTriggerPulled
  (bind _grabbed_interaction_component (Variables|Default|GetGrabbed%20Interaction%20Component))
  (Default|CallOnHandTriggerPulled)
  (if (Variables|Default|GetCanUseTrigger)
    (Variables|Default|SetTriggerPressed_0 true)
    (Variables|Default|SetPullAnchorFound false)
    (Variables|Default|SetBulletHasCollided_0 false)
    (Utilities|IsValid _grabbed_interaction_component
      (:Is%20Valid
        (Default|CallOnTriggerPulled _grabbed_interaction_component)))))

(event EventTriggerRelease
  (bind _grabbed_interaction_component (Variables|Default|GetGrabbed%20Interaction%20Component))
  (Default|CallOnHandTriggerReleased)
  (if (Variables|Default|GetCanUseTrigger)
    (Variables|Default|SetTriggerPressed_0 false)
    (Variables|Default|SetPullAnchorFound false)
    (Variables|Default|SetBulletHasCollided_0 false)
    (Utilities|IsValid _grabbed_interaction_component
      (:Is%20Valid
        (Default|CallOnTriggerReleased _grabbed_interaction_component)))))

(event EventSetWeaponTransform
  (CallFunction|SetWeaponXForm))

(event EventRelease
  (|CallParentFunction)
  (Variables|Default|SetKnifeOffset "0, 0, 0")
  (Variables|Default|SetKnifePitch 0.0)
  (Variables|Default|SetAttachmentComplete false))

(event EventHandHighlightInteractable
  (|CallParentFunction))

(event Input|KeyboardEvents|PageUp
  (params (Key :type Key%20Structure :default "AnyKey"))
  (bind _bone_to_center_to (Variables|Default|GetBone%20to%20center%20to))
  (bind _bone_to_grab (Variables|Default|GetBone%20To%20Grab))
  (bind _bone_to_grab_2 (Variables|Default|GetBone%20To%20Grab))
  (bind _component_to_grab (Variables|Default|GetComponent%20To%20Grab))
  (bind _component_to_grab_2 (Variables|Default|GetComponent%20To%20Grab))
  (bind _main_hand_mesh (Variables|Default|GetMain%20Hand%20Mesh))
  (bind _returnvalue (Transformation|GetSocketTransform _main_hand_mesh _bone_to_center_to "RTS_Component"))
  (bind _returnvalue_2 (Math|Transform|InvertTransform _returnvalue))
  ;[1 1 1] Attach Hand mesh
  (:Pressed
    (Class|SceneComponent|Attachto (Variables|Default|GetMain%20Hand%20Mesh) (Variables|Default|GetScene1) "None" "KeepWorldPosition" false)
    (|SetLerpBackVariables_2_2)
    (Components|Timeline|SetPlayRate (Variables|Default|GetHand%20Lerp) (/ 2.0 (Class|GameplayStatics|GetGlobalTimeDilation)))
    (bind (_direction _position) (Timeline|Timeline_0 ReverseFromEnd)
      (:Update
        (switch Utilities|FlowControl|Switch|SwitchonETimelineDirection _direction
          (:Forward
            (Variables|Default|SetHand%20Lerp%20to%20Transform (Math|Transform|MakeTransform (.location _returnvalue_2) (.rotation _returnvalue_2) (.scale (Variables|Default|GetHand%20Lerp%20from%20Transform))))
            (Transformation|SetWorldTransform (Variables|Default|GetMain%20Hand%20Mesh) (Math|Transform|Lerp(Transform) (Transformation|GetWorldTransform (Variables|Default|GetMain%20Hand%20Mesh)) (Math|Transform|MakeTransform (.location (Math|Transform|ComposeTransforms (Variables|Default|GetHand%20Lerp%20to%20Transform) (select (Transformation|DoesSocketExist _component_to_grab_2 _bone_to_grab) (Transformation|GetSocketTransform _component_to_grab_2 _bone_to_grab "RTS_World") (Transformation|GetWorldTransform (Variables|Default|GetComponent%20To%20Grab))))) (.rotation (Math|Transform|ComposeTransforms (Variables|Default|GetHand%20Lerp%20to%20Transform) (select (Transformation|DoesSocketExist _component_to_grab_2 _bone_to_grab) (Transformation|GetSocketTransform _component_to_grab_2 _bone_to_grab "RTS_World") (Transformation|GetWorldTransform (Variables|Default|GetComponent%20To%20Grab))))) "1,1,1") _position (Utilities|Select :Index _direction :Forward "QuatInterp" :Backward "EulerInterp")) false false))
          (:Backward
            (Transformation|SetRelativeTransform (Variables|Default|GetMain%20Hand%20Mesh) (Math|Transform|Lerp(Transform) (Variables|Default|GetHand%20Lerp%20from%20Transform) (Variables|Default|GetHand%20Lerp%20to%20Transform) _position (Utilities|Select :Index _direction :Forward "QuatInterp" :Backward "EulerInterp")) false false))))
      (:Finished
        (switch Utilities|FlowControl|Switch|SwitchonETimelineDirection _direction
          (:Forward
            (Transformation|AttachComponentToComponent (Variables|Default|GetMain%20Hand%20Mesh) _component_to_grab (select (Transformation|DoesSocketExist _component_to_grab _bone_to_grab_2) _bone_to_grab_2 "") "KeepWorld" "KeepWorld" "KeepWorld" false)
            (Variables|Default|SetAttachmentComplete true)
            (bind _asmistborn_knife (Utilities|Casting|CastToMistbornKnife (Variables|Default|GetGrabbed%20Actor)))
            (Variables|/MistbornMod/Blueprints/Weapon/MistbornKnife.MistbornKnife_C|SetCurrentKnifeOffset _asmistborn_knife 0.0)
            (Variables|/MistbornMod/Blueprints/Weapon/MistbornKnife.MistbornKnife_C|SetCurrentKnifePitch _asmistborn_knife 0.0)))))))

(fn ConstructionScript
  (bind _main_hand_mesh (Variables|Default|GetMain%20Hand%20Mesh))
  (Utilities|FlowControl|Sequence
    (:then_0
      (Class|ActorComponent|SetTickablewhenPaused (Variables|Default|GetWidgetInteraction) true))
    (:then_1
      (bind _output_get (Variables|Default|SetStarting%20Position (+ (* (Math|Transform|InverseTransformLocation (Transformation|GetWorldTransform _main_hand_mesh) (Transformation|GetSocketLocation _main_hand_mesh "b_r_grip")) -1.0) (Variables|Default|GetStarting%20Fudge%20Value))))
      (Transformation|SetRelativeLocation _main_hand_mesh _output_get false false)
      (Variables|Default|SetMain%20Hand%20Mesh%20Starting%20Transform (Transformation|GetRelativeTransform (Variables|Default|GetMain%20Hand%20Mesh))))))

(fn ApplyPullImpulse
  (bind _pullanchoractor (Variables|Default|GetPullAnchorActor))
  (bind _pullanchorpoint (Variables|Default|GetPullAnchorPoint))
  (bind _returnvalue (Transformation|GetActorTransform _pullanchoractor))
  (bind _returnvalue_2 (Math|Transform|TransformLocation _returnvalue _pullanchorpoint))
  (Physics|AddImpulse (Variables|/Script/Engine.Character|GetCharacterMovement (Variables|Default|GetPawn)) (* (Math|Vector|Normalize (- _returnvalue_2 (Transformation|GetWorldLocation (Variables|Default|GetControllerMesh)))) (Variables|Default|GetPullSpeed)) false)
  (Transformation|SetWorldRotation (Variables|Default|GetBlueMetalBeam_0) (Math|Rotator|FindLookatRotation (Transformation|GetWorldLocation (Variables|Default|GetControllerMesh)) _returnvalue_2) false false)
  (Rendering|SetVisibility (Variables|Default|GetBlueMetalBeam_0) true false))

(fn ApplyPullImpulsetoBullet
  (bind _maxpulldistance (Variables|Default|GetMaxPullDistance))
  (bind _bulletcollisionpoint_0 (Variables|Default|GetBulletCollisionPoint_0))
  (bind _controllermesh (Variables|Default|GetControllerMesh))
  (bind _returnvalue (Transformation|GetWorldLocation _controllermesh))
  (bind _returnvalue_2 (- _bulletcollisionpoint_0 _returnvalue))
  (bind _returnvalue_3 (Math|Vector|VectorLength _returnvalue_2))
  (bind _returnvalue_4 (/ _returnvalue_3 _maxpulldistance))
  (bind _returnvalue_5 (Math|Float|Clamp(Float) _returnvalue_4))
  (bind _returnvalue_6 (- 1.0 _returnvalue_5))
  (if (> _returnvalue_3 (Variables|Default|GetMinPullDistance))
    (if (< _returnvalue_3 (Variables|Default|GetMaxPullDistance))
      (Physics|AddImpulse (Variables|/Script/Engine.Character|GetCharacterMovement (Variables|Default|GetPawn)) (* (Math|Vector|Normalize _returnvalue_2) (Variables|Default|GetPullSpeed)) false)
      (Transformation|SetWorldRotation (Variables|Default|GetBlueMetalBeam_0) (Math|Rotator|FindLookatRotation (Transformation|GetWorldLocation (Variables|Default|GetControllerMesh)) (Variables|Default|GetBulletCollisionPoint_0)) false false :!label _label)
      (Rendering|SetVisibility (Variables|Default|GetBlueMetalBeam_0) true false)
      (Transformation|SetRelativeScale3D (Variables|Default|GetBlueMetalBeam_0) (Math|Vector|MakeVector _returnvalue_3 1.0 1.0))
      (Rendering|Material|SetScalarParameterValue (Variables|Default|GetBeamMaterial_0) "LaserOpacity" _returnvalue_6 :!class /Script/Engine.MaterialInstanceDynamic)
      (Class|PlayerController|PlayHapticEffect (Game|GetPlayerController 0) "/Game/Blueprint/Game/FX/ObjectGrabbed.ObjectGrabbed" (Variables|Default|GetHand) (* _returnvalue_6 2.0) false)
      (Variables|Default|SetPullStrength _returnvalue_6)
      (else
        (Variables|Default|SetPullStrength 0.0)
        (Rendering|Material|SetScalarParameterValue (Variables|Default|GetBeamMaterial_0) "LaserOpacity" 0.0 :!class /Script/Engine.MaterialInstanceDynamic)))
    (else
      (Variables|/Script/Engine.MovementComponent|SetVelocity (Variables|/Script/Engine.Character|GetCharacterMovement (Variables|Default|GetPawn)) "0, 0, 0")
      (goto _label))))

(fn HandlePullLogic
  (bind _controllermesh (Variables|Default|GetControllerMesh))
  (bind _grabbed_interaction_component (Variables|Default|GetGrabbed%20Interaction%20Component))
  (bind _returnvalue (Transformation|GetWorldLocation _controllermesh))
  (if (Variables|Default|GetTriggerPressed_0)
    (Utilities|IsValid _grabbed_interaction_component
      (:Is%20Valid
        (Utilities|Casting|CastToMistbornKnife (Components|GetOwner _grabbed_interaction_component)
          (:then
            (if (Variables|Default|GetPullAnchorFound) :!label _label
              (CallFunction|ApplyPullImpulse)
              (else
                (bind (_outhit _returnvalue_2) (Collision|LineTraceByChannel _returnvalue (+ _returnvalue (* (Math|Vector|GetForwardVector _controllermesh) 3e+03)) "TraceTypeQuery2" false (Utilities|Array|MakeArray (Variables|Default|GetPawn)) "None"))
                (if _returnvalue_2
                  (if (Utilities|ClassIsChildOf (Utilities|GetClass (.HitActor (Collision|BreakHitResult _outhit))) "/Game/Character/OdinCharacterBase.OdinCharacterBase_C")
                    (Variables|Default|SetPullAnchorPoint (Math|Transform|InverseTransformLocation (Transformation|GetActorTransform (.HitActor (Collision|BreakHitResult _outhit))) (.ImpactPoint (Collision|BreakHitResult _outhit))))
                    (Variables|Default|SetPullAnchorFound true)
                    (Variables|Default|SetPullAnchorActor (.HitActor (Collision|BreakHitResult _outhit)))
                    (else
                      (Rendering|SetVisibility (Variables|Default|GetBlueMetalBeam_0) false false :!label _label_2)))
                  (else
                    (goto _label_2))))))
          (:CastFailed
            (if (Variables|Default|GetBulletHasCollided_0)
              (CallFunction|ApplyPullImpulsetoBullet)
              (else
                (Variables|Default|SetPullStrength 0.0)
                (Rendering|Material|SetScalarParameterValue (Variables|Default|GetBeamMaterial_0) "LaserOpacity" 0.0 :!class /Script/Engine.MaterialInstanceDynamic))))))
      (:Is%20Not%20Valid
        (goto _label)))
    (else
      (Rendering|SetVisibility (Variables|Default|GetBlueMetalBeam_0) false false)
      (Variables|Default|SetPullStrength 0.0))))

(fn AttachWeapon
  (bind _bone_to_grab (Variables|Default|GetBone%20To%20Grab))
  (bind _component_to_grab (Variables|Default|GetComponent%20To%20Grab))
  (Variables|Default|SetKnifePitch 0.0)
  (CallFunction|SetWeaponXForm)
  (Transformation|AttachComponentToComponent (Variables|Default|GetMain%20Hand%20Mesh) _component_to_grab (select (Transformation|DoesSocketExist _component_to_grab _bone_to_grab) _bone_to_grab "") "KeepWorld" "KeepWorld" "KeepWorld" false))

(fn DetachWeapon
  (Class|SceneComponent|Attachto (Variables|Default|GetMain%20Hand%20Mesh) (Variables|Default|GetScene1) "None" "KeepWorldPosition" false))

(fn SetWeaponXForm
  (bind _returnvalue (Math|Rotator|MakeRotator 9e+01 9e+01 0.0))
  (Utilities|IsValid (Variables|Default|GetGrabbed%20Actor)
    (:Is%20Valid
      (if (and (Variables|Default|GetGrip%20Complete) (Variables|Default|GetGripped))
        (if (and (not (Variables|Default|GetIs%20Secondary%20Grab)) (Class|OdinGrabInteractionComponent|GetPickUponGrab (Variables|Default|GetGrabbed%20Interaction%20Component)))
          (Utilities|FlowControl|Sequence
            (:then_0
              (bind _output_get (LocalVariables|SetIsPhysicsGrab (Utilities|IsValid (Class|PhysicsHandleComponent|GetGrabbedComponent (Variables|Default|GetWeaponPhysicsHandle)))))
              ;[1 1 1] Calculate Grabbed object transform
              (bind _output_get_2 (Variables|Default|SetNew%20Relative%20Transform (CallFunction|CalculateNewRelativeTransform _output_get)))
              (Variables|Default|SetNew%20World%20Transform (CallFunction|CalculateNewWorldTransform _output_get_2)))
            (:then_1
              (if (LocalVariables|GetIsPhysicsGrab)
                ;[1 1 1] Using physics handle, update that
                (Class|PhysicsHandleComponent|SetTargetLocationandRotation (Variables|Default|GetWeaponPhysicsHandle) (.Location (Math|Transform|BreakTransform (Variables|Default|GetNew%20World%20Transform))) (.Rotation (Math|Transform|BreakTransform (Variables|Default|GetNew%20World%20Transform))))
                (else
                  ;[1 1 1] Accounting for recoil on top of laggy hand transform
                  (bind _asgun_base (Utilities|Casting|CastToGun_Base (Variables|Default|GetGrabbed%20Actor))
                    (:then
                      (bind _newguntoworld (Default|ApplyRecoiltoTransform _asgun_base (Variables|Default|GetNew%20Relative%20Transform)))
                      (if (> (.X (Math|Vector|BreakVector (Variables|Default|GetKnifeOffset))) 0.0)
                        (Transformation|SetWorldTransform (VehicleSound|GetRootComponent _asgun_base) (Math|Transform|ComposeTransforms (Math|Transform|MakeTransform (Math|Vector|MakeVector 0.0 0.0 (* (.X (Math|Vector|BreakVector (Variables|Default|GetKnifeOffset))) 1.0)) (Math|Rotator|CombineRotators _returnvalue (Math|Vector|RotatorfromAxisandAngle (Math|Vector|GetRightVector _returnvalue) (Variables|Default|GetKnifePitch))) "1.000000,1.000000,1.000000") (Transformation|GetSocketTransform (Variables|Default|GetMain%20Hand%20Mesh) (Variables|Default|GetBone%20to%20center%20to) "RTS_World")) false false)
                        (else
                          (Transformation|SetRelativeTransform (VehicleSound|GetRootComponent _asgun_base) _newguntoworld false false))))
                    (:CastFailed
                      ;[1 1 1] Not using physics, but not a gun; just set position
                      (Transformation|SetActorTransform (Variables|Default|GetGrabbed%20Actor) (Variables|Default|GetNew%20World%20Transform)))))))
            (:then_2
              (Default|CallOnHandPositionUpdated))))))))

(fn SetKnifeOffset
  (params (NewOffset :type Float%20%28single-precision%29) (NewPitch :type Float%20%28single-precision%29))
  (if (Variables|Default|GetAttachmentComplete)
    (Utilities|FlowControl|Sequence
      (:then_0
        (Variables|Default|SetKnifeOffset (Math|Vector|MakeVector NewOffset 0.0 0.0)))
      (:then_1
        (Variables|Default|SetKnifePitch (* NewPitch 1.0)))
      (:then_2
        (if (> NewOffset 0.0)
          (CallFunction|DetachWeapon)
          (else
            (CallFunction|AttachWeapon)))))))