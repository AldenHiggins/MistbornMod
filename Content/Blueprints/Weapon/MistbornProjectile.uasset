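; MistbornProjectile is a weapon projectile Blueprint that reports its impacts to the push or pull hand linked to it.
; On impact it runs HandleImpact without ricochet, unless a valid InteractionComponent shows it is grabbed.
; After a short delay it passes the hit to the parent push hand, falling back to the pull hand if none is valid.
; Setter events assign both hand references.
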(event Custom|SetParentPushHand
  (params (NewPushHand :type Mistborn%20Hand%20Object%20Reference))
  (Variables|Default|SetParentPushHand NewPushHand))

(event Custom|SetParentPullHand
  (params (NewPullHand :type Mistborn%20Right%20Hand%20Object%20Reference))
  (Variables|Default|SetParentPullHand NewPullHand))

(event EventNotifyProjectileImpact
  (params (Hit :type Hit%20Result%20Structure%20%28by%20ref%29) (NormalImpulse :type Vector :default "0, 0, 0"))
  (bind _interaction_component (Variables|Default|GetInteraction%20Component))
  (bind _parentpushhand (Variables|Default|GetParentPushHand))
  (bind _parentpullhand (Variables|Default|GetParentPullHand))
  (Utilities|IsValid _interaction_component
    (:Is%20Valid
      (if (not (Class|OdinGrabInteractionComponent|GetIsGrabbed _interaction_component))
        (CallFunction|HandleImpact Hit false :!label _label)
        (Utilities|FlowControl|Delay 0.2)
        (Utilities|IsValid _parentpushhand
          (:Is%20Valid
            (Default|PushedBulletCollision _parentpushhand 0 0 "0, 0, 0" Hit))
          (:Is%20Not%20Valid
            (Utilities|IsValid _parentpullhand
              (:Is%20Valid
                (Default|PulledBulletCollision _parentpullhand Hit)))))))
    (:Is%20Not%20Valid
      (goto _label))))

(fn ConstructionScript
  (|CallParentFunction))