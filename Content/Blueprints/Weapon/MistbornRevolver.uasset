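; Revolver weapon Blueprint for the Mistborn pawn, extending a parent weapon class that handles spawning bullets.
; After each shot it casts the owning pawn to MistbornPawn and reports the last spawned bullet and the primary grabbing hand as the recently fired bullet.
; On BeginPlay it overrides the sight and ammo cylinder materials.
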(event EventBeginPlay
  ;[1 1 1] Override the sight/cylinder materials on spawn
  (|CallParentFunction)
  (Rendering|Material|SetMaterial (Variables|Default|Getsight) 0 (Variables|Default|GetSightMaterial))
  (Rendering|Material|SetMaterial (Variables|Default|GetAmmo) 0 (Variables|Default|GetAmmoMaterial)))

(event EventSpawnBullets
  ;[1 1 1] Notify the pawn that we've fired a bullet
  (|CallParentFunction)
  (bind _asmistborn_pawn (Utilities|Casting|CastToMistbornPawn (Variables|Default|GetOwning%20Pawn)))
  (Default|SetRecentlyFiredBullet _asmistborn_pawn (Variables|Default|GetLastSpawnedBullet) (Variables|Default|GetPrimary%20Grabbing%20Hand)))

(fn ConstructionScript
  (|CallParentFunction))