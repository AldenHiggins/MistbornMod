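; Blueprint child that swaps its inherited holsters for Mistborn holster components when play begins.
; BeginPlay assigns the left, right, back-right and back-left Mistborn components to the parent's two leg and two back holster variables.
; The assignments run before the parent BeginPlay, so inherited setup sees the overrides, while the construction script only calls the parent.
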(event EventBeginPlay
  ;[1 1 1] Override holsters with our mistborn holsters on spawn
  (Variables|Default|SetLeg%20Left%20Holster (Variables|Default|GetMistbornHolsterComponentLeft))
  (Variables|Default|SetLeg%20Right%20Holster (Variables|Default|GetMistbornHolsterComponentRight))
  (Variables|Default|SetBack%20Right%20Holster (Variables|Default|GetMistbornHolsterComponentBackRight))
  (Variables|Default|SetBack%20Left%20Holster (Variables|Default|GetMistbornHolsterComponentBackLeft))
  (|CallParentFunction))

(fn ConstructionScript
  (|CallParentFunction))