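; Child gun Blueprint for a Mistborn bullet weapon, carrying ten visible bullets gathered into an array on BeginPlay.
; Each shot hides the next bullet and reports the spawned bullet and firing hand to the owning MistbornPawn.
; Ending the grab enables physics on every bullet in the array, hides the pickup haze and blocks further pickup.
; Empty overrides suppress the parent's throw-for-grabbing and out-of-ammo UI animation events.
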(event EventBeginPlay
  (bind _bullets (Variables|Default|GetBullets))
  (|CallParentFunction)
  (Utilities|Array|Add _bullets (Variables|Default|GetBullet1))
  (Utilities|Array|Add _bullets (Variables|Default|GetBullet2))
  (Utilities|Array|Add _bullets (Variables|Default|GetBullet3))
  (Utilities|Array|Add _bullets (Variables|Default|GetBullet4))
  (Utilities|Array|Add _bullets (Variables|Default|GetBullet5))
  (Utilities|Array|Add _bullets (Variables|Default|GetBullet6))
  (Utilities|Array|Add _bullets (Variables|Default|GetBullet7))
  (Utilities|Array|Add _bullets (Variables|Default|GetBullet8))
  (Utilities|Array|Add _bullets (Variables|Default|GetBullet9))
  (Utilities|Array|Add _bullets (Variables|Default|GetBullet10)))

(event EventBndEvtPrimaryInteractionComponentK2NodeComponentBoundEvent61onEndInteractionDelegateDelegateSignature
  (params (InteractionComponent :type Odin%20Grab%20Interaction%20Component%20Object%20Reference) (ReleasingMotionController :type Motion%20Controller%20Component%20Object%20Reference) (ReleasingHandActor :type Actor%20Object%20Reference) (Hand :type EControllerHand%20Enum :default "Left"))
  (|CallParentFunction 0 0 0 "Left")
  (for _array_element (Variables|Default|GetBullets)
    (Physics|SetSimulatePhysics _array_element true)
    (Variables|Default|SetCan%20Be%20Picked%20Up false)
    (Rendering|SetVisibility (Variables|Default|GetPickupHazeMesh) false false)
    (Class|OdinGrabInteractionComponent|SetAllowInteraction (Variables|Default|GetPrimary%20Interaction%20Component) false)))

(event EventSpawnBullets
  (bind _bullets (Variables|Default|GetBullets))
  (bind _bulletsfired (Variables|Default|GetBulletsFired))
  (|CallParentFunction)
  (if (> (Utilities|Array|Length _bullets) _bulletsfired)
    (Rendering|SetVisibility (Utilities|Array|Get(acopy) _bullets _bulletsfired) false false)
    (Math|Integer|IncrementInt (Variables|Default|GetBulletsFired)
      (:%20%20
        (bind _asmistborn_pawn (Utilities|Casting|CastToMistbornPawn (Variables|Default|GetOwning%20Pawn)))
        (Default|SetRecentlyFiredBullet _asmistborn_pawn (Variables|Default|GetLastSpawnedBullet) (Variables|Default|GetPrimary%20Grabbing%20Hand))))))

(event EventPlayOutOfAmmoUIAnim)

(event EventThrowGunforGrabbing
  (params (AI%20Drop :type Boolean)))

(fn ConstructionScript
  (|CallParentFunction))