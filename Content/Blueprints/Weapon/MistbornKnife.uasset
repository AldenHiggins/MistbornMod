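; VR knife weapon that deals melee damage to Odin and drone characters, overriding its parent's ammo and firing behavior.
; Hits count when held or moving fast enough, then start a timeline-driven cooldown.
; Holding the trigger grows an offset and accumulating pitch fed to MistbornHand, easing the offset back on release.
; Fast releases enable throw flight, which zeroes spin and aligns the knife to its velocity until it collides.
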(event OnComponentHit(WeapMesh)
  (params (HitComponent :type Primitive%20Component%20Object%20Reference) (OtherActor :type Actor%20Object%20Reference) (OtherComp :type Primitive%20Component%20Object%20Reference) (NormalImpulse :type Vector :default "0, 0, 0") (Hit :type Hit%20Result%20Structure%20%28by%20ref%29))
  (CallFunction|KnifeComponentHit OtherActor))

(event Custom|RevolverFired
  ;[1 1 1] Simple Overrides
)

(event EventBndEvtPrimaryInteractionComponentK2NodeComponentBoundEvent31onTriggerPulledDelegateSignature
  (Variables|Default|SetTriggerPressed true))

(event EventBndEvtPrimaryInteractionComponentK2NodeComponentBoundEvent46onTriggerReleasedDelegateSignature
  (Variables|Default|SetTriggerPressed false))

(event EventPlayOutOfAmmoUIAnim
  ;[1 1 1] Simple Overrides
  (Utilities|FlowControl|Delay 0.2))

(event EventNotifyFired
  ;[1 1 1] Simple Overrides
  (Utilities|FlowControl|Delay 0.2))

(event EventRefillAmmo
  ;[1 1 1] Simple Overrides
)

(event EventUpdateAmmoCounter
  ;[1 1 1] Simple Overrides
)

(event EventBndEvtPrimaryInteractionComponentK2NodeComponentBoundEvent61onEndInteractionDelegateDelegateSignature
  (params (InteractionComponent :type Odin%20Grab%20Interaction%20Component%20Object%20Reference) (ReleasingMotionController :type Motion%20Controller%20Component%20Object%20Reference) (ReleasingHandActor :type Actor%20Object%20Reference) (Hand :type EControllerHand%20Enum :default "Left"))
  ;[1 1 1] On Throw
  (Utilities|FlowControl|Sequence
    (:then_0
      (bind _asbp_default_hand (Utilities|Casting|CastToBP_DefaultHand ReleasingHandActor))
      (if (>= (Math|Vector|VectorLengthSquared (.World%20Space%20Velocity (Default|GetVelocity (Variables|/Game/Character/Player/Avatars/BP_DefaultHand.BP_DefaultHand_C|GetVelocityTrackingComponent _asbp_default_hand)))) (Variables|Default|GetThrowingSpeedThreshold))
        (Variables|Default|SetEnableVelocityFollowing true)))
    (:then_1
      (|CallParentFunction InteractionComponent ReleasingMotionController ReleasingHandActor Hand))))

(event EventAnimNotifyEnterFireIdle
  ;[1 1 1] Simple Overrides
  (Utilities|FlowControl|Delay 0.2))

(event EventPlayUIShotFiredAnim
  ;[1 1 1] Simple Overrides
  (Utilities|FlowControl|Delay 0.2))

(event EventBeginPrimaryGrab
  ;[1 1 1] Simple Overrides
  (Rendering|SetVisibility (Variables|Default|GetAmmoCounter) false false))

(event EventBndEvtPrimaryInteractionComponentK2NodeComponentBoundEvent4onBeginInteractionDelegateDelegateSignature
  (params (InteractionComponent :type Odin%20Grab%20Interaction%20Component%20Object%20Reference) (GrabbingMotionController :type Motion%20Controller%20Component%20Object%20Reference) (GrabbingHandActor :type Actor%20Object%20Reference) (Hand :type EControllerHand%20Enum) (GrabbedComponent :type Primitive%20Component%20Object%20Reference))
  ;[1 1 1] On Grab
  (|CallParentFunction InteractionComponent GrabbingMotionController GrabbingHandActor Hand GrabbedComponent)
  (Variables|Default|SetCurrentKnifePitch 0.0)
  (Variables|Default|SetCurrentKnifeOffset 0.0))

(event EventTick
  (params (DeltaSeconds :type Float%20%28single-precision%29))
  ;[1 1 1] On Tick
  (|CallParentFunction 0.0)
  (CallFunction|ThrowTick)
  (CallFunction|HeldTick DeltaSeconds)
  (if (and (Variables|Default|GetCollisionCoolDown) (not (Variables|Default|GetCollisionCoolDownInProgress)))
    (Variables|Default|SetCollisionCoolDownInProgress true)
    (Timeline|Timeline_2 PlayFromStart
      (:Finished
        (Variables|Default|SetCollisionCoolDown false)
        (Variables|Default|SetCollisionCoolDownInProgress false)))))

(fn ConstructionScript
  (|CallParentFunction))

(fn KnifeComponentHit
  (params (OtherActor :type Actor%20Object%20Reference))
  (if (not (Variables|Default|GetCollisionCoolDown))
    (Utilities|FlowControl|Sequence
      (:then_0
        (if (Physics|IsSimulatingPhysics (Variables|Default|GetWeapMesh) "None")
          (Variables|Default|SetHasCollided true)))
      (:then_1
        (if (or (>= (Math|Vector|VectorLengthSquared (Transformation|GetComponentVelocity (Variables|Default|GetWeapMesh))) (Variables|Default|GetMeleeVelocityThreshold)) (not (Physics|IsSimulatingPhysics (Variables|Default|GetWeapMesh) "None")))
          (Variables|Default|SetCollisionCoolDown true)
          (Utilities|FlowControl|Sequence
            (:then_0
              (bind _asodin_character_base (Utilities|Casting|CastToOdinCharacterBase OtherActor))
              (Utilities|IsValid _asodin_character_base
                (:Is%20Valid
                  (Game|Damage|ApplyDamage _asodin_character_base (Variables|Default|GetMeleeDamage) 0 0 "/Game/Blueprint/DamageTypes/DamageType_Melee.DamageType_Melee_C"))))
            (:then_1
              (bind _asdrone_character_base (Utilities|Casting|CastToDroneCharacterBase OtherActor))
              (Utilities|IsValid _asdrone_character_base
                (:Is%20Valid
                  (Game|Damage|ApplyDamage _asdrone_character_base (Variables|Default|GetMeleeDamage) 0 0 "/Game/Blueprint/DamageTypes/DamageType_Melee.DamageType_Melee_C"))))))))))

(fn ThrowTick
  (bind _weapmesh (Variables|Default|GetWeapMesh))
  (bind _returnvalue (Transformation|GetComponentVelocity _weapmesh))
  (bind _returnvalue_2 (Math|Rotator|MakeRotfromX _returnvalue))
  (if (Math|Boolean|ANDBoolean (Physics|IsSimulatingPhysics (Variables|Default|GetWeapMesh) "None") (Variables|Default|GetEnableVelocityFollowing) (not (Variables|Default|GetHasCollided)))
    (Class|PrimitiveComponent|SetPhysicsAngularVelocity (Variables|Default|GetWeapMesh) "0, 0, 0" false "None")
    (Transformation|SetWorldRotation (Variables|Default|GetVelocityArrow) _returnvalue_2 false false)
    (Transformation|SetActorRotation (Math|Rotator|CombineRotators "-80.000000,0.000000, 0" _returnvalue_2) true)))

(fn HeldTick
  (params (DeltaTime :type Float%20%28single-precision%29))
  (bind _knifeoffsetgrowthspeed (Variables|Default|GetKnifeOffsetGrowthSpeed))
  (bind _returnvalue (* _knifeoffsetgrowthspeed DeltaTime))
  (if (and (Class|OdinGrabInteractionComponent|GetIsGrabbed (Variables|Default|GetPrimary%20Interaction%20Component)) (or (> (Variables|Default|GetCurrentKnifeOffset) 0.0) (Variables|Default|GetTriggerPressed)))
    (Utilities|FlowControl|Sequence
      (:then_0
        (if (Variables|Default|GetTriggerPressed)
          (Variables|Default|SetCurrentKnifeOffset (Math|Float|Min(Float) (+ (Variables|Default|GetCurrentKnifeOffset) _returnvalue) (Variables|Default|GetMaxKnifeDistance)))
          (else
            (Variables|Default|SetCurrentKnifeOffset (Math|Float|Max(Float) (- (Variables|Default|GetCurrentKnifeOffset) _returnvalue) 0.0)))))
      (:then_1
        (Variables|Default|SetCurrentKnifePitch (+ (Variables|Default|GetCurrentKnifePitch) (* (Variables|Default|GetPitchGrowthRate) (Variables|Default|GetCurrentKnifeOffset)))))
      (:then_2
        (bind _asmistborn_hand (Utilities|Casting|CastToMistbornHand (Variables|Default|GetGrabbing%20Hand%20Blueprint)))
        (Default|SetKnifeOffset _asmistborn_hand (Variables|Default|GetCurrentKnifeOffset) (Variables|Default|GetCurrentKnifePitch))))))