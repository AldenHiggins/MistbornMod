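; Mistborn holster component that spawns and refreshes the gun held in a player's back or leg holster.
; Refreshing replaces any held gun with the override class or the re-holstered weapon, restoring the latter's saved ammo, and flags left or right from holster type.
; The gun attaches with interaction and shadows off and collision suppressed.
; A separate event starts the reload cooldown and broadcasts it.
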(event EventRefreshGun
  (params (Pawn :type Pawn%20Object%20Reference))
  (CallFunction|RefreshMistbornGun Pawn))

(event EventStartCooldown
  (if (Variables|Default|GetbIsRefreshEnabled)
    (Variables|Default|SetbHolsterRefreshed false)
    (bind _output_get (Variables|Default|SetHolsterRefreshCooldown (Variables|Default|GetGunReloadCooldown)))
    (Variables|Default|SetHolsterRefreshCooldownStart _output_get)
    (Default|CallOnCooldownStart)))

(fn RefreshMistbornGun
  (params (Pawn :type Pawn%20Object%20Reference))
  (if (Variables|Default|GetbIsRefreshEnabled)
    (if (Variables|Default|GetbHasGun)
      ;[1 1 1] If gun already is in holster, replenish ammo for it
      (Actor|DestroyActor (Variables|Default|GetGunReference))
      (Variables|Default|SetGunReference 0))
    (LocalVariables|SetPawn%20Instigator Pawn)
    (LocalVariables|SetGun%20Class (Variables|Default|GetGunClassOverride))
    (if (Variables|Default|GetbReHolsteredWeapon)
      (LocalVariables|SetGun%20Class (Variables|Default|GetReholsteredGun)))
    (bind _asgun_base (Utilities|Casting|CastToGun_BaseClass (LocalVariables|GetGun%20Class)))
    (Variables|Default|SetHolsterGunClass _asgun_base)
    (switch Utilities|FlowControl|Switch|SwitchonELoadoutSlotTypes (Variables|Default|GetType)
      (:BackLeft
        (Variables|Default|SetbOnLeft true :!label _label))
      (:BackRight
        (Variables|Default|SetbOnLeft false :!label _label_2))
      (:LegLeft
        (goto _label))
      (:LegRight
        (goto _label_2)))
    (bind _returnvalue (Game|SpawnActorfromClass _asgun_base (Transformation|GetWorldTransform) "AlwaysSpawn" 0 true false (Variables|Default|GetbWeapModified) (Variables|Default|GetbOnLeft) (LocalVariables|GetPawn%20Instigator)))
    (bind _output_get (Variables|Default|SetGunReference _returnvalue))
    (Variables|Default|SetGun_PreviewMesh (Variables|/Game/Prototype/Game/Gun_Base.Gun_Base_C|GetWeapMesh _output_get))
    (Variables|Default|SetLoadoutWeaponName (Variables|/Game/Prototype/Game/Gun_Base.Gun_Base_C|GetWeaponName _output_get))
    (EventDispatchers|BindEventtoOnDropped _returnvalue (EventDispatchers|CreateEvent :!event OnDropped))
    (EventDispatchers|BindEventtoGrabbed _returnvalue (EventDispatchers|CreateEvent :!event OnGrabbed))
    (if (Variables|Default|GetbReHolsteredWeapon)
      (Variables|/Script/Odin.OdinWeapon|SetAmmoRemaining (Variables|Default|GetGunReference) (Variables|Default|GetBulletsRemaining))
      (Default|UpdateAmmoCounter (Variables|Default|GetGunReference)))
    (Collision|SetCollisionEnabled (.AsPrimitive%20Component (Utilities|Casting|CastToPrimitiveComponent (Components|GetChildComponent (Variables|/Game/Prototype/Game/Gun_Base.Gun_Base_C|GetPrimary%20Interaction%20Component (Variables|Default|GetGunReference)) 0))) "NoCollision")
    (Transformation|AttachComponentToComponent (Variables|Default|GetGunReference) self "None" "SnapToTarget" "SnapToTarget" "SnapToTarget" false)
    (bind _primary (Default|GetPrimaryandSecondaryOverlaps (Variables|Default|GetGunReference)))
    (Collision|SetCollisionProfileName _primary "OdinIgnoreAll" :!class /Script/Engine.PrimitiveComponent)
    (Class|OdinGrabInteractionComponent|SetAllowInteraction (Variables|/Game/Prototype/Game/Gun_Base.Gun_Base_C|GetPrimary%20Interaction%20Component (Variables|Default|GetGunReference)) false)
    (Variables|Default|SetbHasGun true)
    (Default|RemovePreviewMeshComponent (Variables|Default|GetParentHolsters) (Variables|Default|GetGun_PreviewMeshComponent))
    (Rendering|SetCastShadow (Variables|/Game/Prototype/Game/Gun_Base.Gun_Base_C|GetWeapMesh (Variables|Default|GetGunReference)) false)
    (Default|CallRefreshedGun)))